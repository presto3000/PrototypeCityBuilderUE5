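; Camera pawn for a grid building-placement game, with screen-edge scrolling, axis-input movement and a starting stock of four coloured building types.
; BeginPlay caches the player controller and refreshes its building counts; MovingGhostBuilding grid-snaps a ghost building under the cursor.
; Spawning, placement, scoring by tile colour and neighbour bonus, and end-game logic sit in unwired chains that never run, leaving their events empty.
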(event Custom|MovingGhostBuilding
  (bind _returnvalue (Game|GetPlayerController 0))
  (bind _array (Utilities|Array|MakeArray "ObjectTypeQuery1"))
  (bind (_hitresult _returnvalue_2) (Class|PlayerController|GetHitResultUnderCursorforObjects _returnvalue _array true))
  (bind _location (Collision|BreakHitResult _hitresult))
  (bind (_x _y _z) (Math|Vector|BreakVector _location))
  ;[1 1 1] SpawnGhostBuilding
  (Utilities|IsValid (Variables|Default|GetGhostBuilding)
    (:Is%20Valid
      (if (and _returnvalue_2 (not (.ReturnValue (Class|PlayerController|GetHitResultUnderCursorforObjects (Game|GetPlayerController 0) (Utilities|Array|MakeArray "ObjectTypeQuery2") true))))
        (Variables|Default|SetHitPlaneActorClass (Utilities|GetClass (.HitActor (Collision|BreakHitResult _hitresult))))
        (Transformation|SetActorLocation (Variables|Default|GetGhostBuilding) (Math|Vector|MakeVector (Math|Float|SnapToGrid(Float) _x 1e+02) (Math|Float|SnapToGrid(Float) _y 1e+02) _z) false false)))))

(event Custom|SpawnGhostBuilding
  (params (InGhostBuilding :type BP%20Master%20Ghost%20Building%20Class%20Reference))
  ;[1 1 1] SpawnGhostBuilding
)

(event Custom|SpawnActualBuilding
  (params (InBuildingClass :type BP%20Master%20Building%20Class%20Reference) (InTransform :type Transform)))

(event Custom|SetActualBuilding
  (params (InActualBuilding :type BP%20Master%20Building%20Class%20Reference)))

(event Custom|BuildingPlaced)

(event Custom|DestroyGhost)

(event EventBeginPlay
  ;[1 1 1] BeginPlay
  (bind _asbp_player_controller (Utilities|Casting|CastToBP_PlayerController (Game|GetPlayerController 0)))
  (Variables|Default|SetAs%20BP%20Player%20Controller _asbp_player_controller)
  (Default|OnBuildingAmountUpdated (Variables|Default|GetAs%20BP%20Player%20Controller)))

(event Collision|EventActorBeginOverlap
  (params (OtherActor :type Actor%20Object%20Reference)))

(event EventTick
  (params (DeltaSeconds :type Float%20%28single-precision%29)))

(event Input|AxisEvents|InputAxisMoveForwardBackwardCamera
  (params (AxisValue :type Float%20%28single-precision%29))
  ;[1 1 1] WASD
  (Transformation|AddActorLocalOffset (Math|Vector|MakeVector 0.0 0.0 (* AxisValue (Variables|Default|GetCamera_MoveSpeed))) true false))

(event Input|AxisEvents|InputAxisMoveRightLeftCamera
  (params (AxisValue :type Float%20%28single-precision%29))
  ;[1 1 1] WASD
  (Transformation|AddActorLocalOffset (Math|Vector|MakeVector 0.0 (* AxisValue (Variables|Default|GetCamera_MoveSpeed)) 0.0) true false))

(event Input|MouseEvents|MouseX
  (params (AxisValue :type Float%20%28single-precision%29))
  (bind _returnvalue (Game|GetPlayerController 0))
  (bind _returnvalue_2 (Viewport|GetViewportSize))
  (bind _returnvalue_3 (Utilities|Time|GetWorldDeltaSeconds))
  (bind _scroll_speed (Variables|Default|GetScroll%20Speed))
  (bind _locationx (Game|Player|GetMousePosition _returnvalue))
  (bind _returnvalue_4 (* _scroll_speed _returnvalue_3))
  (bind _returnvalue_5 (/ _locationx (.x _returnvalue_2)))
  ;[1 1 1] EDGE SCROLLING
  (if (> _returnvalue_5 0.98)
    (Transformation|AddActorWorldOffset (Math|Vector|MakeVector 0.0 _returnvalue_4 0.0))
    (elif (< _returnvalue_5 0.02)
      (Transformation|AddActorWorldOffset (Math|Vector|MakeVector 0.0 (* _returnvalue_4 -1.0) 0.0)))))

(event Input|MouseEvents|MouseY
  (params (AxisValue :type Float%20%28single-precision%29))
  (bind _returnvalue (Game|GetPlayerController 0))
  (bind _returnvalue_2 (Viewport|GetViewportSize))
  (bind _returnvalue_3 (Utilities|Time|GetWorldDeltaSeconds))
  (bind _scroll_speed (Variables|Default|GetScroll%20Speed))
  (bind _locationy (Game|Player|GetMousePosition _returnvalue))
  (bind _returnvalue_4 (* _scroll_speed _returnvalue_3))
  (bind _returnvalue_5 (/ _locationy (.y _returnvalue_2)))
  ;[1 1 1] EDGE SCROLLING
  (if (> _returnvalue_5 0.98)
    (Transformation|AddActorWorldOffset (Math|Vector|MakeVector (* _returnvalue_4 -1.0) 0.0 0.0))
    (elif (< _returnvalue_5 0.02)
      (Transformation|AddActorWorldOffset (Math|Vector|MakeVector _returnvalue_4 0.0 0.0)))))

(event Input|MouseEvents|LeftMouseButton
  (params (Key :type Key%20Structure :default "None")))

(event Input|MouseEvents|RightMouseButton
  (params (Key :type Key%20Structure :default "None")))

(fn ConstructionScript
  (Variables|Default|SetRedBuildingsAmount 3)
  (Variables|Default|SetYellowBuildingsAmount 3)
  (Variables|Default|SetWhiteBuildingsAmount 3)
  (Variables|Default|SetPurpleBuildingsAmount 3))

(fn CheckHittedBuildings
  (params (InGhostBuilding :type BP%20Master%20Ghost%20Building%20Object%20Reference))
  (bind _hitactorclassone (Variables|/Game/_DEV/Blueprints/Buildings/GhostBuildings/BP_MasterGhostBuilding.BP_MasterGhostBuilding_C|GetHitActorClassOne InGhostBuilding))
  (bind _hitactorclasstwo (Variables|/Game/_DEV/Blueprints/Buildings/GhostBuildings/BP_MasterGhostBuilding.BP_MasterGhostBuilding_C|GetHitActorClassTwo InGhostBuilding))
  (bind _hitactorclassthree (Variables|/Game/_DEV/Blueprints/Buildings/GhostBuildings/BP_MasterGhostBuilding.BP_MasterGhostBuilding_C|GetHitActorClassThree InGhostBuilding))
  (bind _hitactorclassfour (Variables|/Game/_DEV/Blueprints/Buildings/GhostBuildings/BP_MasterGhostBuilding.BP_MasterGhostBuilding_C|GetHitActorClassFour InGhostBuilding))
  (Utilities|FlowControl|Sequence
    (:then_0
      (if (== _hitactorclassone "/Game/_DEV/Blueprints/Buildings/BP_BuildingWhite.BP_BuildingWhite_C")
        (LocalVariables|SetCounterWhite (+ (LocalVariables|GetCounterWhite) 1))
        (elif (== _hitactorclassone "/Game/_DEV/Blueprints/Buildings/BP_BuildingYellow.BP_BuildingYellow_C")
          (LocalVariables|SetCounterYellow (+ (LocalVariables|GetCounterYellow) 1))
          (elif (== _hitactorclassone "/Game/_DEV/Blueprints/Buildings/BP_BuildingRed.BP_BuildingRed_C")
            (LocalVariables|SetCounterRed (+ (LocalVariables|GetCounterRed) 1))
            (elif (== _hitactorclassone "/Game/_DEV/Blueprints/Buildings/BP_BuildingPurple.BP_BuildingPurple_C")
              (LocalVariables|SetCounterPurple (+ (LocalVariables|GetCounterPurple) 1)))))))
    (:then_1
      (if (== _hitactorclasstwo "/Game/_DEV/Blueprints/Buildings/BP_BuildingWhite.BP_BuildingWhite_C")
        (LocalVariables|SetCounterWhite (+ (LocalVariables|GetCounterWhite) 1))
        (elif (== _hitactorclasstwo "/Game/_DEV/Blueprints/Buildings/BP_BuildingYellow.BP_BuildingYellow_C")
          (LocalVariables|SetCounterYellow (+ (LocalVariables|GetCounterYellow) 1))
          (elif (== _hitactorclasstwo "/Game/_DEV/Blueprints/Buildings/BP_BuildingRed.BP_BuildingRed_C")
            (LocalVariables|SetCounterRed (+ (LocalVariables|GetCounterRed) 1))
            (elif (== _hitactorclasstwo "/Game/_DEV/Blueprints/Buildings/BP_BuildingPurple.BP_BuildingPurple_C")
              (LocalVariables|SetCounterPurple (+ (LocalVariables|GetCounterPurple) 1)))))))
    (:then_2
      (if (== _hitactorclassthree "/Game/_DEV/Blueprints/Buildings/BP_BuildingWhite.BP_BuildingWhite_C")
        (LocalVariables|SetCounterWhite (+ (LocalVariables|GetCounterWhite) 1))
        (elif (== _hitactorclassthree "/Game/_DEV/Blueprints/Buildings/BP_BuildingYellow.BP_BuildingYellow_C")
          (LocalVariables|SetCounterYellow (+ (LocalVariables|GetCounterYellow) 1))
          (elif (== _hitactorclassthree "/Game/_DEV/Blueprints/Buildings/BP_BuildingRed.BP_BuildingRed_C")
            (LocalVariables|SetCounterRed (+ (LocalVariables|GetCounterRed) 1))
            (elif (== _hitactorclassthree "/Game/_DEV/Blueprints/Buildings/BP_BuildingPurple.BP_BuildingPurple_C")
              (LocalVariables|SetCounterPurple (+ (LocalVariables|GetCounterPurple) 1)))))))
    (:then_3
      (if (== _hitactorclassfour "/Game/_DEV/Blueprints/Buildings/BP_BuildingWhite.BP_BuildingWhite_C")
        (LocalVariables|SetCounterWhite (+ (LocalVariables|GetCounterWhite) 1))
        (elif (== _hitactorclassfour "/Game/_DEV/Blueprints/Buildings/BP_BuildingYellow.BP_BuildingYellow_C")
          (LocalVariables|SetCounterYellow (+ (LocalVariables|GetCounterYellow) 1))
          (elif (== _hitactorclassfour "/Game/_DEV/Blueprints/Buildings/BP_BuildingRed.BP_BuildingRed_C")
            (LocalVariables|SetCounterRed (+ (LocalVariables|GetCounterRed) 1))
            (elif (== _hitactorclassfour "/Game/_DEV/Blueprints/Buildings/BP_BuildingPurple.BP_BuildingPurple_C")
              (LocalVariables|SetCounterPurple (+ (LocalVariables|GetCounterPurple) 1)))))))
    (:then_4
      (if (and (> (LocalVariables|GetCounterYellow) 0) (> (LocalVariables|GetCounterRed) 0))
        (LocalVariables|SetMultiplierPlus 3.0)
        (elif (and (> (LocalVariables|GetCounterRed) 0) (> (LocalVariables|GetCounterWhite) 0))
          (LocalVariables|SetMultiplierPlus 2.0)
          (elif (and (> (LocalVariables|GetCounterRed) 0) (> (LocalVariables|GetCounterPurple) 0))
            (LocalVariables|SetMultiplierPlus -2.0)
            (elif (and (> (LocalVariables|GetCounterYellow) 0) (> (LocalVariables|GetCounterWhite) 0))
              (LocalVariables|SetMultiplierPlus 3.0)
              (elif (and (> (LocalVariables|GetCounterYellow) 0) (> (LocalVariables|GetCounterPurple) 0))
                (LocalVariables|SetMultiplierPlus -1.0)
                (elif (and (> (LocalVariables|GetCounterWhite) 0) (> (LocalVariables|GetCounterPurple) 0))
                  (LocalVariables|SetMultiplierPlus 1.0)
                  (else
                    (LocalVariables|SetMultiplierPlus 0.0))))))))
      (return (LocalVariables|GetMultiplierPlus)))))