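; Player controller Blueprint for a building-placement score game, holding UI logic that is currently disconnected, so all its events are empty.
; The orphaned chains would create the overlay widget from the camera pawn and refresh its score and per-color building counts.
; Another orphaned chain would show an end-game window with the final score and a fade-in animation.
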(event Custom|ShowEndGameWindow)

(event EventBeginPlay)

(event EventTick
  (params (DeltaSeconds :type Float%20%28single-precision%29)))

(event EventOnScoreUpdated)

(event EventOnBuildingAmountUpdated)

(fn ConstructionScript)